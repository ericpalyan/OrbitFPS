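; BP_Box_TEST is a test box actor that changes its material parameters at runtime.
; BeginPlay creates a dynamic material instance on the Box component's first slot.
; Overlap begin and end both apply the same moss ground texture and Opacity value, so leaving does not revert the change.
; A ToggleVsibility event sets a lower Opacity on that instance without toggling back.
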(event `self.ReceiveActorBeginOverlap`
  (params (OtherActor :type "Actor Object Reference"))
  (bind _mid (`self.MID`))
  (`MaterialInstanceDynamic.SetTextureParameterValue` _mid "BaseColor" "/Game/Textures/T_Ground_Moss_D.T_ground_Moss_D")
  (`MaterialInstanceDynamic.SetScalarParameterValue` _mid "Opacity" 2.5))

(event `self.ReceiveActorEndOverlap`
  (params (OtherActor :type "Actor Object Reference"))
  (bind _mid (`self.MID`))
  (`MaterialInstanceDynamic.SetTextureParameterValue` _mid "BaseColor" "/Game/Textures/T_Ground_Moss_D.T_ground_Moss_D")
  (`MaterialInstanceDynamic.SetScalarParameterValue` _mid "Opacity" 2.5))

(event `self.ReceiveBeginPlay`
  (bind _returnvalue (`PrimitiveComponent.CreateDynamicMaterialInstance` (`self.Box`) 0 null))
  (set `self.MID` _returnvalue))

(event `ToggleVsibility`
  (`MaterialInstanceDynamic.SetScalarParameterValue` (`self.MID`) "Opacity" 0.5))

(fn `UserConstructionScript`)