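; Broken wall sconce that flickers while something overlaps its Proximity component, then dies and smokes when the overlap ends.
; A looping random Delay toggles LightBulb and BounceLight visibility while IsWithinProximity and IsNotBroken hold.
; Leaving turns both lights off, clears IsNotBroken, then after a short delay shows PSmoke and toggles SmokeAudio.
; Later overlaps re-enter the broken branch, so they can toggle the smoke audio again.
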(event `self.Proximity.OnComponentBeginOverlap`
  (params (OtherActor :type "Actor Object Reference") (OtherComp :type "PrimitiveComponent Object Reference") (OtherBodyIndex :type Integer))
  (set `self.isWithinProximity` true)
  (if (`self.isWithinProximity`) :!label _label
    (if (and (`self.isWithinProximity`) (`self.isNotBroken`)) :!label _label_2
      (`KismetSystemLibrary.Delay` (`KismetMathLibrary.RandomFloatInRange` 0.0 0.6))
      (`SceneComponent.ToggleVisibility` (`self. LightBulb`) false)
      (`SceneComponent.ToggleVisibility` (`self.BounceLight`) false)
      (goto _label_2)
      (else
        _)))
  (`SceneComponent.SetVisibility` (`self. LightBulb`) false false)
  (`SceneComponent.SetVisibility` (`self.BounceLight`) false false)
  (set `self.isNotBroken` false)
  (`KismetSystemLibrary.Delay` 0.2)
  (`ActorComponent.ToggleActive` (`self.Smoke Audio`))
  (`SceneComponent.SetVisibility` (`self.P_Smoke`) true false))

(event `self.Proximity.OnComponentEndOverlap`
  (params (OtherActor :type "Actor Object Reference") (OtherComp :type "PrimitiveComponent Object Reference") (OtherBodyIndex :type Integer))
  (set `self.isWithinProximity` false)
  (goto _label))

(fn `UserConstructionScript`)