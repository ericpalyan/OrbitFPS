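; Player controller for the Orbit game that toggles the HUD and lets a player without a pawn respawn.
; It caches BP_Orbit_HUD on BeginPlay and forwards EnableHUD calls to it.
; The Respawn input calls RequestRespawn only when no valid pawn is controlled.
; RequestRespawn acts only with authority, asking BP_Orbit_GameMode to respawn this controller with the Random option set.
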(event `self.ReceiveBeginPlay`
  (bind _asbp_orbit_hud_c (cast `/Game/Blueprints/BP_Orbit_HUD` (`self.GetHUD` self)))
  (set `self.HUD` _asbp_orbit_hud_c))

(event `Enable HUD`
  (params (Enable :type Boolean))
  (bind _hud (`self.HUD`))
  (if Enable
    (`/Game/Blueprints/BP_Orbit_HUD.Enable HUD` _hud)
    (else
      (`/Game/Blueprints/BP_Orbit_HUD.Disable HUD` _hud))))

(event `InputAction|Respawn`
  (:`Pressed`
    (`/Engine/EditorBlueprintResources/StandardMacros.IsValid` (`self.GetControlledPawn`)
      (:`Is Not Valid`
        (`self.RequestRespawn`)))))

(event `RequestRespawn`
  (bind _returnvalue (`GameplayStatics.GetGameMode`))
  (`/Engine/EditorBlueprintResources/ActorMacros.Switch Has Authority`
    (:`Authority`
      (`/Engine/EditorBlueprintResources/StandardMacros.IsValid` _returnvalue
        (:`Is Valid`
          (bind _asbp_orbit_gamemode_c (cast `/Game/Blueprints/BP_Orbit_GameMode` _returnvalue))
          (`/Engine/EditorBlueprintResources/StandardMacros.IsValid` _asbp_orbit_gamemode_c
            (:`Is Valid`
              (bind _returnvalue_2 (`self.CastToPlayerController`))
              (`/Game/Blueprints/BP_Orbit_GameMode.Respawn` :`self` _asbp_orbit_gamemode_c :`Controller` _returnvalue_2 :`Random` true))))))))

(fn `UserConstructionScript`)