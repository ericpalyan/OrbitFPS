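; Player controller Blueprint that lets a player request a respawn through the Respawn input action.
; The input acts only with authority and when no valid pawn is controlled, then calls RequestRespawn.
; RequestRespawn checks authority again, casts the game mode to MyGame, and delegates to its Respawn function with the random option enabled.
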(event `InputAction|Respawn`
  (:`Pressed`
    (`/Engine/EditorBlueprintResources/ActorMacros.Switch Has Authority`
      (:`Authority`
        (`/Engine/EditorBlueprintResources/StandardMacros.IsValid` (`self.GetControlledPawn`)
          (:`Is Not Valid`
            (`self.RequestRespawn`)))))))

(event `RequestRespawn`
  (bind _returnvalue (`GameplayStatics.GetGameMode`))
  (`/Engine/EditorBlueprintResources/ActorMacros.Switch Has Authority`
    (:`Authority`
      (`/Engine/EditorBlueprintResources/StandardMacros.IsValid` _returnvalue
        (:`Is Valid`
          (bind _asmygame_c (cast `/Game/Blueprints/MyGame` _returnvalue))
          (`/Engine/EditorBlueprintResources/StandardMacros.IsValid` _asmygame_c
            (:`Is Valid`
              (`self.CastToPlayerController`)
              (`/Game/Blueprints/MyGame.Respawn` :`self` _asmygame_c :`Random` true))))))))

(fn `UserConstructionScript`)